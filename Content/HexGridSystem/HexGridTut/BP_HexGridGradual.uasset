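; Hex grid terrain generator that builds a noise-driven tile map on BeginPlay and rebuilds it with random seeds on Left Ctrl release.
; Two FastNoise layers set each instanced tile's height and custom data, with optional flat water and scaled depths.
; Staggered rows come from a FlipFlop; a non-instanced mode spawns child-actor tiles without height.
; The delayed-loop gradual spawn is disconnected, so the grid builds at once.
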(event `self.ReceiveBeginPlay`
  (bind _noise_scale (`self.Noise Scale`))
  (bind _lvl_2_noise_scale (`self.Lvl 2 Noise Scale`))
  (bind _outinstancetransform (`InstancedStaticMeshComponent.GetInstanceTransform` (`self.InstancedStaticMesh`) (`self.InstanceIndex`) true))
  (bind _returnvalue (`FastNoiseWrapper.GetNoise2D` (`self.NoiseWrapperLvl1`) (* (.x (.location _outinstancetransform)) _noise_scale) (* (.y (.location _outinstancetransform)) _noise_scale)))
  (bind _returnvalue_2 (+ _returnvalue (`KismetMathLibrary.FClamp` (`FastNoiseWrapper.GetNoise2D` (`self.NoiseWrapperLvl2`) (* (.x (.location _outinstancetransform)) _lvl_2_noise_scale) (* (.y (.location _outinstancetransform)) _lvl_2_noise_scale)) -1.0)))
  (`self.EnableInput` (`GameplayStatics.GetPlayerController` 0))
  ;[1 1 1] Construct Noise Level 1
  (bind _returnvalue_3 (`|GenericCreateObject` "/Script/FastNoiseGenerator.FastNoiseWrapper" :!label _label))
  (bind _output_get (set `self.NoiseWrapperLvl1` _returnvalue_3))
  (`FastNoiseWrapper.SetupFastNoise` _output_get (`self.Noise Type`) (`self.Seed`) (`self.Frequency`) (`self.Interp`) (`self.Fractaltype`) (`self.Octaves`) (`self.Lacunarity`) (`self.Gain`) (`self.Cellular Jitter`) (`self.Cellular Distance Function`) (`self.Cellular Return Type`))
  ;[1 1 1] Construct Noise Level 2
  (bind _returnvalue_4 (`|GenericCreateObject` "/Script/FastNoiseGenerator.FastNoiseWrapper"))
  (bind _output_get_2 (set `self.NoiseWrapperLvl2` _returnvalue_4))
  (`FastNoiseWrapper.SetupFastNoise` _output_get_2 (`self.Lvl 2 Noise Type`) (`self.Lvl 2 Seed`) (`self.Lvl 2 Frequency`) (`self.Lvl 2 Interp`) (`self.Lvl 2 Fractaltype`) (`self.Lvl 2 Octaves`) (`self.Lvl 2 Lacunarity`) (`self.Lvl 2 Gain`) (`self.Lvl 2 Cellular Jitter`) (`self.Lvl 2 Cellular Distance Function`) (`self.Lvl 2 Cellular Return Type_0`))
  (`StaticMeshComponent.SetStaticMesh` (`self.InstancedStaticMesh`) (`self.TileMesh`))
  (set `self.Radius` (* (.x (`.Max` (break `Box` (`StaticMesh.GetBoundingBox` (`self.TileMesh`))))) (`self.Scale`)))
  ;[1 1 1] Height Loop
  (for _index (range (`self.Height`))
    ;[1 1 1] Width Loop
    (for _index_2 (range (`self.Width`))
      (if (`self.Instanced?`)
        (bind _returnvalue_5 (+ (* _index_2 (`self.Radius`) 2.0) (* _index_2 (`self.Offset`)) (`self.RowOffset`)))
        (bind _returnvalue_6 (+ (* (/ (* (`self.Radius`) 2.0) (`KismetMathLibrary.Sqrt` 3.0)) 1.5 _index) (* _index (`self.Offset`))))
        ;[1 1 1] Instanced Mesh
        (bind _returnvalue_7 (`InstancedStaticMeshComponent.AddInstance` (`self.InstancedStaticMesh`) (`KismetMathLibrary.MakeTransform` (`KismetMathLibrary.MakeVector` _returnvalue_5 _returnvalue_6) (struct) (`KismetMathLibrary.Conv_DoubleToVector` (`self.Scale`))) false))
        (`KismetMaterialLibrary.SetScalarParameterValue` "/Game/HexGridSystem/Material/MPC_HexGrid.MPC_HexGrid" "WaterThreshold" (`self.Water Threshold`))
        ;[1 1 1] Randomize Tile Height
        (set `self.InstanceIndex` _returnvalue_7)
        (if (and (<= _returnvalue (`self.Water Threshold`)) (`self.bFlatWaterTiles`))
          ;[1 1 1] Flat Water Tile Settings
          (set `self.TileHeight` (+ (`self.Water Threshold`) (`self.BaseWaterHeight`)))
          (elif (< _returnvalue_2 0.0)
            (set `self.TileHeight` (* (`self.WaterDepthMultiplier`) _returnvalue_2))
            (else
              (set `self.TileHeight` _returnvalue_2))))
        (`InstancedStaticMeshComponent.UpdateInstanceTransform` (`self.InstancedStaticMesh`) (`self.InstanceIndex`) (`KismetMathLibrary.MakeTransform` (+ (.location (`InstancedStaticMeshComponent.GetInstanceTransform` (`self.InstancedStaticMesh`) (`self.InstanceIndex`) true)) (`KismetMathLibrary.MakeVector` 0.0 0.0 (+ (* (+ (`self.TileHeight`) 0.0) (`self.TileHeightStrength`)) (`self.TileHeightOffset`)))) (struct) (`KismetMathLibrary.Conv_DoubleToVector` (`self.Scale`))) true false false)
        (`InstancedStaticMeshComponent.SetCustomDataValue` (`self.InstancedStaticMesh`) (`self.InstanceIndex`) 0 (`self.TileHeight`) true)
        (else
          ;[1 1 1] Child Actors
          (bind _returnvalue_8 (`AddComponent|NODE_AddChildActorComponent-1` :`RelativeTransform` (`KismetMathLibrary.MakeTransform` (`KismetMathLibrary.MakeVector` _returnvalue_5 _returnvalue_6) (struct) (`KismetMathLibrary.Conv_DoubleToVector` (`self.Scale`)))))
          (`ChildActorComponent.SetChildActorClass` _returnvalue_8 "/Game/HexGridSystem/HexGridTut/BP_Tile.BP_Tile_C")
          (bind _asbp_hex_tile (cast `/Game/HexGridSystem/BP_HexTile` (`ChildActorComponent.ChildActor` _returnvalue_8)))
          (`StaticMeshComponent.SetStaticMesh` (`/Game/HexGridSystem/BP_HexTile.HexTile` _asbp_hex_tile) (`self.TileMesh`)))))
    (`/Engine/EditorBlueprintResources/StandardMacros.FlipFlop`
      (:`A`
        (set `self.RowOffset` (* (`self.Radius`) -1.0)))
      (:`B`
        (set `self.RowOffset` 0.0))))
  (`SceneComponent.SetWorldScale3D` (`self.StaticMesh`) (`KismetMathLibrary.MakeVector` (`KismetMathLibrary.Conv_IntToDouble` (`self.Width`)) (* (`KismetMathLibrary.Conv_IntToDouble` (`self.Height`)) 0.75) 1.0)))

(event `Respawn Grid`
  (`InstancedStaticMeshComponent.ClearInstances` (`self.InstancedStaticMesh`))
  (goto _label))

(event `Key|LeftControl`
  (params (Key :type "Key Structure"))
  (:`Released`
    (bind _output_get (set `self.Seed` (`KismetMathLibrary.RandomIntegerInRange` 0 99999)))
    (bind _output_get_2 (set `self.Lvl 2 Seed` (`KismetMathLibrary.RandomIntegerInRange` 0 99999)))
    (`self.Respawn Grid`)
    (`KismetSystemLibrary.PrintString` (`KismetStringLibrary.Concat_StrStr` "Seed 1: " (`KismetStringLibrary.Conv_IntToString` _output_get) "; Seed 2: " (`KismetStringLibrary.Conv_IntToString` _output_get_2)) true true (struct :`R` 1.0 :`B` 0.065193 :`A` 1.0))))

(fn `UserConstructionScript`
  (locals (InstanceIndex :type Integer :default 0)))