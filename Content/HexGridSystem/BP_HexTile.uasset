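; BP_HexTile is a hex grid tile actor that shows its terrain type and responds to mouse hover and clicks.
; The construction script creates a dynamic material and starts the tile as Empty; UpdateHex drives its Generated? and LandType parameters for water, grass or forest, using Height only for grass.
; Hover swaps cursor and highlight color.
; Click release toggles a locked highlight and a W_TilePopup widget placed relative to the mouse.
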(event `self.ReceiveActorOnReleased`
  (params (ButtonReleased :type "Key Structure"))
  (bind _popupwidget (`self.PopUpWidget`))
  (bind (_locationx _locationy) (`PlayerController.GetMousePosition` (`GameplayStatics.GetPlayerController` 0)))
  (`/Engine/EditorBlueprintResources/StandardMacros.FlipFlop`
    (:`A`
      (set `self.MouseClicked?` true)
      (`MeshComponent.SetVectorParameterValueOnMaterials` (`self.HexTile`) "EmptyColor" (`KismetMathLibrary.Conv_LinearColorToVector` (`self.HighlightColor`)))
      (bind _returnvalue (`|CreateWidget` "/Game/Widgets/W_TilePopup.W_TilePopup_C"))
      (bind _output_get (set `self.PopUpWidget` _returnvalue))
      (`UserWidget.AddToViewport` _output_get 0)
      (`UserWidget.SetDesiredSizeInViewport` _popupwidget (250.0 350.0))
      (`UserWidget.SetPositionInViewport` _popupwidget (`KismetMathLibrary.MakeVector2D` (- _locationx 300.0) (- _locationy 175.0)) true))
    (:`B`
      (set `self.MouseClicked?` false)
      (`MeshComponent.SetVectorParameterValueOnMaterials` (`self.HexTile`) "EmptyColor" (`KismetMathLibrary.Conv_LinearColorToVector` (`self.EmptyColor`)))
      (`Widget.RemoveFromParent` (`self.PopUpWidget`)))))

(event `self.ReceiveActorBeginCursorOver`
  (if (not (`self.MouseClicked?`))
    (set `PlayerController.CurrentMouseCursor` "Hand" (`GameplayStatics.GetPlayerController` 0))
    (`MeshComponent.SetVectorParameterValueOnMaterials` (`self.HexTile`) "EmptyColor" (`KismetMathLibrary.Conv_LinearColorToVector` (`self.HighlightColor`)))))

(event `self.ReceiveActorEndCursorOver`
  (if (not (`self.MouseClicked?`))
    (set `PlayerController.CurrentMouseCursor` "Default" (`GameplayStatics.GetPlayerController` 0))
    (`MeshComponent.SetVectorParameterValueOnMaterials` (`self.HexTile`) "EmptyColor" (`KismetMathLibrary.Conv_LinearColorToVector` (`self.EmptyColor`)))))

(event `UpdateHex`
  (params (Height :type "Float (double-precision)") (Biome :type "Float (double-precision)") (`Water/Land` :type "Float (double-precision)") (HexType :type "/Game/HexGridSystem/Material/E_HexTileTypes Enum" :default "NewEnumerator0"))
  (switch `/Game/HexGridSystem/Material/E_HexTileTypes` HexType
    (:`NewEnumerator4`
      (`MeshComponent.SetScalarParameterValueOnMaterials` (`self.HexTile`) "Generated?" 0.0))
    (:`NewEnumerator0`
      (`MeshComponent.SetVectorParameterValueOnMaterials` (`self.HexTile`) "LandType" (0.0 0.0 0.0))
      (`MeshComponent.SetScalarParameterValueOnMaterials` (`self.HexTile`) "Generated?" 1.0 :!label _label))
    (:`NewEnumerator1`
      (`MeshComponent.SetVectorParameterValueOnMaterials` (`self.HexTile`) "LandType" (`KismetMathLibrary.MakeVector` Height 0.0 1.0))
      (goto _label))
    (:`NewEnumerator2`
      (`MeshComponent.SetVectorParameterValueOnMaterials` (`self.HexTile`) "LandType" (0.0 1.0 1.0))
      (goto _label))))

(event `self.ReceiveBeginPlay`)

(fn `UserConstructionScript`
  (bind _returnvalue (`PrimitiveComponent.CreateDynamicMaterialInstance` (`self.HexTile`) 0 "/Game/HexGridSystem/M_PlanetDefault.M_PlanetDefault" "None"))
  (set `self.HexMaterial` _returnvalue)
  (`self.UpdateHex` 0.0 0.0 0.0 "NewEnumerator4"))