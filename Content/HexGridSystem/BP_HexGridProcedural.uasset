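; Procedural planet actor that builds a noise-displaced cube sphere in the construction script when Update is set, despite its hex grid name.
; ConstructPlanes rotates six welded grids into cube faces, normalizes their vertices onto a scaled sphere and offsets them with per-axis 1D Perlin noise.
; Each face becomes a procedural mesh section with the planet material, and VerticesDefault keeps all generated vertices.
; An AddNoise helper is defined but not called here.
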(fn `AddNoise`
  (params (A :type "Vector Structure"))
  (returns (ReturnValue :type "Vector Structure"))
  (bind (_returnvalue_x _returnvalue_y _returnvalue_z) (`KismetMathLibrary.BreakVector` (+ A (`self.NoiseOffset`))))
  (return (* (+ (`KismetAnimationLibrary.K2_MakePerlinNoiseVectorAndRemap` _returnvalue_x _returnvalue_y _returnvalue_z -1.0 1.0 -1.0 "1.f" -1.0) (`self.ShapePull`)) (`self.Noise Scale`))))

(fn `ConstructPlanes`
  (locals (Index :type Integer))
  (bind _resolution (`self.Resolution`))
  (if (`self.Update`)
    (`KismetArrayLibrary.Array_Clear` (`self.Vertices(Default)`))
    (for _index (range 6)
      (set `local.Index` _index)
      (bind (_triangles _vertices _uvs) (`KismetProceduralMeshLibrary.CreateGridMeshWelded` _resolution _resolution 1.0))
      (set `self.Triangles` _triangles)
      (set `self.UVs` _uvs)
      (for _array_element _vertices
        (bind _returnvalue (`KismetMathLibrary.Normal` (`KismetMathLibrary.GreaterGreater_VectorRotator` (+ _array_element (`KismetMathLibrary.MakeVector` 0.0 0.0 (/ (- (`self.Resolution`) 1) 2.0))) (`|GetArrayItem` (`self.FaceRotations`) (`local.Index`)))))
        (bind (_x _y _z) (`KismetMathLibrary.BreakVector3f` _returnvalue))
        (bind _returnvalue_2 (+ (* _returnvalue (`self.Scale`)) (* (`KismetMathLibrary.MakeVector` (`KismetMathLibrary.PerlinNoise1D` _x) (`KismetMathLibrary.PerlinNoise1D` _y) (`KismetMathLibrary.PerlinNoise1D` _z)) (/ (`self.Scale`) 4))))
        (`KismetArrayLibrary.Array_Add` (`self.Vertices`) _returnvalue_2)
        (`KismetArrayLibrary.Array_Add` (`self.Vertices(Default)`) _returnvalue_2))
      (`PrimitiveComponent.SetMaterial` (`self.ProceduralMesh`) (`local.Index`) "/Game/HexGridSystem/M_PlanetDefault.M_PlanetDefault")
      (`ProceduralMeshComponent.CreateMeshSection_LinearColor` :`self` (`self.ProceduralMesh`) :`SectionIndex` (`local.Index`) :`Vertices` (`self.Vertices`) :`Triangles` (`self.Triangles`) :`UV0` (`self.UVs`))
      (`KismetArrayLibrary.Array_Clear` (`self.Vertices`)))))

(fn `UserConstructionScript`
  (`self.ConstructPlanes`))