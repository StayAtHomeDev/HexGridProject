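; BP_Tile is a tile in the hex grid system that randomizes its own elevation as terrain or water.
; Its construction script picks either the base water height or a clamped random height, offsets the mesh vertically by the scaled value, and passes it to the material's Elevation parameter.
; BeginPlay is empty, and the random color and timeline-driven glow logic is disconnected.
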(event `self.ReceiveBeginPlay`)

(fn `UserConstructionScript`
  (bind _returnvalue (`KismetMathLibrary.RandomFloatInRange` -1.0 1.0))
  (bind _staticmesh (`self.StaticMesh`))
  ;[1 1 1] Calculate Height
  (if (<= _returnvalue 0.0)
    (set `self.Height` (`self.Base Water Height`))
    (else
      (set `self.Height` (`KismetMathLibrary.FClamp` _returnvalue 0.1))))
  (`SceneComponent.K2_SetWorldLocation` _staticmesh (+ (`SceneComponent.K2_GetComponentLocation` _staticmesh) (`KismetMathLibrary.MakeVector` 0.0 0.0 (+ (* (`self.Height`) (`self.Strength`)) (`self.Offset`)))) false false)
  (`MeshComponent.SetScalarParameterValueOnMaterials` (`self.StaticMesh`) "Elevation" (`self.Height`)))